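; BP_Character is a character Blueprint that handles background music and pause menu toggling.
; On BeginPlay it starts the music as a 2D sound and keeps a reference to it.
; The PauseGame input flips a flag, creating a new WBP_PauseMenu or removing it while switching game pause, music pause, cursor visibility and input mode.
; Opening uses Game and UI input, and closing restores Game Only.
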(event EventBeginPlay
  (bind _returnvalue (Audio|SpawnSound2D "/Game/Assets/Sound/Background_Music_Cue.Background_Music_Cue" 1.0 1.0 0.0 0))
  (Variables|Default|Set2DSound _returnvalue))

(event Collision|EventActorBeginOverlap
  (params (OtherActor :type Actor%20Object%20Reference)))

(event EventTick
  (params (DeltaSeconds :type Float%20%28single-precision%29)))

(event Input|ActionEvents|InputActionPauseGame
  (params (Key :type Key%20Structure :default "None"))
  (bind _returnvalue (Game|GetPlayerController 0))
  (bind _returnvalue_2 (Game|GetPlayerController 0))
  (:Pressed
    (if (Variables|Default|GetIsPauseMenuOpen)
      (Widget|RemovefromParent (stale _returnvalue_3))
      (Input|SetInputModeGameOnly _returnvalue_2 false)
      (Variables|/Script/Engine.PlayerController|SetbShowMouseCursor _returnvalue_2 false)
      (Game|SetGamePaused false)
      (Class|AudioComponent|SetPaused (Variables|Default|Get2DSound) false)
      (Variables|Default|SetIsPauseMenuOpen false)
      (else
        (bind _returnvalue_3 (UserInterface|CreateWidget "/Game/Blueprints/Game/WBP_PauseMenu.WBP_PauseMenu_C"))
        (UserInterface|Viewport|AddtoViewport _returnvalue_3 0)
        (Game|SetGamePaused true)
        (Input|SetInputModeGameandUI _returnvalue 0 "DoNotLock" true false)
        (Variables|/Script/Engine.PlayerController|SetbShowMouseCursor _returnvalue true)
        (Class|AudioComponent|SetPaused (Variables|Default|Get2DSound) true)
        (Variables|Default|SetIsPauseMenuOpen true)))))

(fn ConstructionScript)